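; Road tile for an endless runner that spawns random coins and animates a hazard car along a spline with a timeline.
; Coin rolls are nested, so the right spawn requires the center one and the left requires the right.
; The player overlapping Box has the game mode spawn new ground and add a point, raises walk speed within a clamp, then destroys the tile after a delay.
; Overlapping Box1 or DangerZone kills the player.
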(event OnComponentBeginOverlap(Box)
  (params (OverlappedComponent :type Primitive%20Component%20Object%20Reference) (OtherActor :type Actor%20Object%20Reference) (OtherComp :type Primitive%20Component%20Object%20Reference) (OtherBodyIndex :type Integer) (bFromSweep :type Boolean) (SweepResult :type Hit%20Result%20Structure%20%28by%20ref%29))
  (Utilities|Casting|CastToThirdPersonCharacter OtherActor)
  (bind _asthird_person_game_mode (Utilities|Casting|CastToThirdPersonGameMode (Game|GetGameMode)))
  (Default|SpawnGround _asthird_person_game_mode)
  (bind _asthird_person_game_mode_2 (Utilities|Casting|CastToThirdPersonGameMode (Game|GetGameMode)))
  (Variables|/Game/ThirdPersonBP/Blueprints/ThirdPersonGameMode.ThirdPersonGameMode_C|Setcurrentpoint _asthird_person_game_mode_2 (+ (Variables|/Game/ThirdPersonBP/Blueprints/ThirdPersonGameMode.ThirdPersonGameMode_C|Getcurrentpoint _asthird_person_game_mode_2) 1))
  (bind _asthird_person_character (Utilities|Casting|CastToThirdPersonCharacter (Game|GetPlayerCharacter 0)))
  (Variables|/Script/Engine.CharacterMovementComponent|SetMaxWalkSpeed (Variables|/Script/Engine.Character|GetCharacterMovement _asthird_person_character) (Math|Float|Clamp(Float) (* (Variables|/Script/Engine.CharacterMovementComponent|GetMaxWalkSpeed (Variables|/Script/Engine.Character|GetCharacterMovement _asthird_person_character)) 1.02) 4e+02 8e+02))
  (Utilities|FlowControl|Delay 1.0)
  (Actor|DestroyActor))

(event OnComponentBeginOverlap(Box1)
  (params (OverlappedComponent :type Primitive%20Component%20Object%20Reference) (OtherActor :type Actor%20Object%20Reference) (OtherComp :type Primitive%20Component%20Object%20Reference) (OtherBodyIndex :type Integer) (bFromSweep :type Boolean) (SweepResult :type Hit%20Result%20Structure%20%28by%20ref%29))
  (bind _asthird_person_character (Utilities|Casting|CastToThirdPersonCharacter OtherActor))
  (Default|Death _asthird_person_character))

(event OnComponentBeginOverlap(dangerZone)
  (params (OverlappedComponent :type Primitive%20Component%20Object%20Reference) (OtherActor :type Actor%20Object%20Reference) (OtherComp :type Primitive%20Component%20Object%20Reference) (OtherBodyIndex :type Integer) (bFromSweep :type Boolean) (SweepResult :type Hit%20Result%20Structure%20%28by%20ref%29))
  (bind _asthird_person_character (Utilities|Casting|CastToThirdPersonCharacter OtherActor))
  (Default|Death _asthird_person_character))

(event EventBeginPlay
  (CallFunction|CoinSpawn)
  (bind _newtrack_0 (Timeline|moveBluecar Play)
    (:Update
      (Transformation|SetWorldLocation (Variables|Default|Getcar) (Spline|GetLocationatDistanceAlongSpline (Variables|Default|GetSpline) (* _newtrack_0 (Spline|GetSplineLength (Variables|Default|GetSpline))) "World") false false))))

(event Collision|EventActorBeginOverlap
  (params (OtherActor :type Actor%20Object%20Reference)))

(event EventTick
  (params (DeltaSeconds :type Float%20%28single-precision%29)))

(fn ConstructionScript)

(fn CoinSpawn
  ;[1 1 1] left line
  (switch int (Math|Random|RandomIntegerinRange 0 1)
    (:1
      (Game|SpawnActorfromClass "/Game/assets/coin/coin_pickup.coin_pickup_C" (Transformation|GetWorldTransform (Variables|Default|Getcenter)) "Undefined" 0 0)
      ;[1 1 1] right lane
      (switch int (Math|Random|RandomIntegerinRange 0 2)
        (:1
          (Game|SpawnActorfromClass "/Game/assets/coin/coin_pickup.coin_pickup_C" (Transformation|GetWorldTransform (Variables|Default|Getright)) "Undefined" 0 0)
          ;[1 1 1] center lane
          (switch int (Math|Random|RandomIntegerinRange 0 2)
            (:1
              (Game|SpawnActorfromClass "/Game/assets/coin/coin_pickup.coin_pickup_C" (Transformation|GetWorldTransform (Variables|Default|Getleft)) "Undefined" 0 0))))))))